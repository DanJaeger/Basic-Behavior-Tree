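; BP_NPC_Character is an NPC character Blueprint that supplies patrol destinations and adjustable walk speed.
; On BeginPlay it gathers every BP_PatrolPoint actor in the level into PatrolPoints.
; UpdatePatrolPoint cycles an index through that array and returns the actor's location, incrementing before reading, so the index can reach one past the end.
; UpdateWalkSpeed sets the movement component's MaxWalkSpeed.
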(event EventBeginPlay
  (bind _outactors (Actor|GetAllActorsOfClass "/Game/Blueprints/BP_PatrolPoint.BP_PatrolPoint_C"))
  (Variables|Default|SetPatrolPoints _outactors))

(fn ConstructionScript)

(fn UpdateWalkSpeed
  (params (NewWalkSpeed :type Float%20%28double-precision%29))
  (Variables|/Script/Engine.CharacterMovementComponent|SetMaxWalkSpeed (Variables|Character|GetCharacterMovement) NewWalkSpeed))

(fn UpdatePatrolPoint
  (if (Utilities|Array|IsNotEmpty (Variables|Default|GetPatrolPoints))
    (if (< (Variables|Default|GetCurrentPatrolPoint) (Utilities|Array|Length (Variables|Default|GetPatrolPoints)))
      (Math|Integer|IncrementInt (Variables|Default|GetCurrentPatrolPoint)
        (:%20%20
          (return (Transformation|GetActorLocation (Utilities|Array|Get(acopy) (Variables|Default|GetPatrolPoints) (Variables|Default|GetCurrentPatrolPoint))))))
      (else
        (Variables|Default|SetCurrentPatrolPoint 0)
        (return (Transformation|GetActorLocation (Utilities|Array|Get(acopy) (Variables|Default|GetPatrolPoints) (Variables|Default|GetCurrentPatrolPoint))))))))